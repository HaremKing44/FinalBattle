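; Player knight character with camera-relative movement, sprinting, rolling, blocking and sword combat.
; A sword spawns on a holder socket; equipping locks input during the montage and switches to controller-facing rotation, enabling attack, block and eight-way montage rolls.
; Light attacks chain up to four hits through an Anim Blueprint callback, notifying the sword when to deal damage.
; Tick maintains the block montage and eases walk speed back to normal.
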(event `self.ReceiveBeginPlay`
  (bind _returnvalue (`|SpawnActorFromClass` (`self.WeaponClass`) (`SceneComponent.GetSocketTransform` (`self.Mesh`) "SwordHolderSocket" "RTS_World") "Undefined" "OverrideRootScale" null null))
  (set `self.WeaponObject` _returnvalue)
  (`self.K2_AttachToComponent` (`self.WeaponObject`) (`self.Mesh`) "SwordHolderSocket" "SnapToTarget" "SnapToTarget" "SnapToTarget" true)
  (set `self.IsWeaponEquiped` false)
  (bind _asbp_sword (cast `/Game/Blueprints/Weapon/BP_Sword` (`self.WeaponObject`)))
  (set `self.CastedWeaponObject` _asbp_sword))

(event `self.ReceiveTick`
  (params (DeltaSeconds :type "Float (single-precision)"))
  (`|ExecutionSequence`
    (:`then_0`
      (if (or (`self.isSprinting`) (`self.isBlocking`))
        _
        (elif (not (`KismetMathLibrary.InRange_FloatFloat` (`self.Max Walk Speed`) 299.0 301.0))
          (bind _output_get (set `self.Max Walk Speed` (`KismetMathLibrary.Lerp` (`self.Max Walk Speed`) 300.0 0.1)))
          (`self.ChangePlayerWalkspeed` _output_get))))
    (:`then_1`
      (`self.Play Block Animation`))))

(event `InputAxis|MoveForward`
  (params (AxisValue :type "Float (single-precision)"))
  (bind (_returnvalue_roll _returnvalue_pitch _returnvalue_yaw) (`KismetMathLibrary.BreakRotator` (`self.GetControlRotation`)))
  ;[1 1 1] Character Movement
  (bind _output_get (set `self.InputAxisForward` AxisValue))
  (`self.AddMovementInput` (`KismetMathLibrary.GetForwardVector` (`KismetMathLibrary.MakeRotator` 0.0 0.0 _returnvalue_yaw)) _output_get))

(event `InputAxis|MoveRight`
  (params (AxisValue :type "Float (single-precision)"))
  (bind (_returnvalue_roll _returnvalue_pitch _returnvalue_yaw) (`KismetMathLibrary.BreakRotator` (`self.GetControlRotation`)))
  ;[1 1 1] Character Movement
  (bind _output_get (set `self.InputAxisRight` AxisValue))
  (`self.AddMovementInput` (`KismetMathLibrary.GetRightVector` (`KismetMathLibrary.MakeRotator` 0.0 0.0 _returnvalue_yaw)) _output_get))

(event `InputAction|Sprint`
  (params (Key :type "Key Structure"))
  ;[1 1 1] Control Character Sprint
  (:`Pressed`
    (bind _returnvalue (`KismetSystemLibrary.K2_SetTimerDelegate` (delegate `CheckCanSprint`) 0.2 true)))
  (:`Released`
    (set `self.isSprinting` false)
    (`KismetSystemLibrary.K2_ClearAndInvalidateTimerHandle` _returnvalue)))

(event `CheckCanSprint`
  ;[1 1 1] Control Character Sprint
  (if (and (> (`self.InputAxisForward`) 0.0) (== (`self.InputAxisRight`) 0.0))
    (set `self.isSprinting` true)
    (bind _output_get (set `self.Max Walk Speed` 450.0))
    (`self.ChangePlayerWalkspeed` _output_get)
    (else
      (set `self.isSprinting` false))))

(event `InputAxis|Turn`
  (params (AxisValue :type "Float (single-precision)"))
  ;[1 1 1] Character Camera Movement with mouse and Gamepad
  (`self.AddControllerYawInput` AxisValue))

(event `InputAxis|LookUp`
  (params (AxisValue :type "Float (single-precision)"))
  ;[1 1 1] Character Camera Movement with mouse and Gamepad
  (`self.AddControllerPitchInput` AxisValue))

(event `InputAxis|TurnRate`
  (params (AxisValue :type "Float (single-precision)"))
  ;[1 1 1] Character Camera Movement with mouse and Gamepad
  (`self.AddControllerYawInput` (* AxisValue (`GameplayStatics.GetWorldDeltaSeconds`) (`self.TurnRate`))))

(event `InputAxis|LookUpRate`
  (params (AxisValue :type "Float (single-precision)"))
  ;[1 1 1] Character Camera Movement with mouse and Gamepad
  (`self.AddControllerPitchInput` (* AxisValue (`GameplayStatics.GetWorldDeltaSeconds`) (`self.LookUpRate`))))

(event `InputAction|Equip/UneQuip`
  (params (Key :type "Key Structure"))
  (bind _charactermovement (`self.CharacterMovement`))
  ;[1 1 1] Equip/UnequipWeapon
  (:`Pressed`
    (if (not (`self.isRolling`))
      (if (`self.IsWeaponEquiped`)
        (`self.PlayAnimMontage` "/Game/GKnight/Animation/Swordman_Montage/Equip/A_SW_Unequip_Trim_Montage.A_SW_Unequip_Trim_Montage")
        (bind _output_get (set `self.isPlayerInputEnable` false))
        (`self.TogglePlayerInput` _output_get)
        (`KismetSystemLibrary.RetriggerableDelay` 1.6)
        (bind _output_get_2 (set `self.isPlayerInputEnable` true))
        (`self.TogglePlayerInput` _output_get_2)
        (set `self.IsWeaponEquiped` false)
        (set `CharacterMovementComponent.bOrientRotationToMovement` true _charactermovement)
        (set `self.bUseControllerRotationYaw` false)
        (`self.ResetCombat`)
        (else
          (`self.PlayAnimMontage` "/Game/GKnight/Animation/Swordman_Montage/Equip/A_SW_Equip_Montage.A_SW_Equip_Montage")
          (bind _output_get_3 (set `self.isPlayerInputEnable` false))
          (`self.TogglePlayerInput` _output_get_3)
          (`KismetSystemLibrary.RetriggerableDelay` 1.8)
          (bind _output_get_4 (set `self.isPlayerInputEnable` true))
          (`self.TogglePlayerInput` _output_get_4)
          (set `self.IsWeaponEquiped` true)
          (set `CharacterMovementComponent.bOrientRotationToMovement` false _charactermovement)
          (set `self.bUseControllerRotationYaw` true))))))

(event `InputAction|Roll`
  (params (Key :type "Key Structure"))
  ;[1 1 1] Roll
  (:`Pressed`
    (if (`self.IsWeaponEquiped`)
      (`/Engine/EditorBlueprintResources/StandardMacros.DoOnce` false :!label _label
        (:`Completed`
          (set `self.isRolling` true)
          (bind (_forward _right) (`self.GetDesiredDirectionForRoll`))
          (`self.ChooseRollAnimation` _forward _right)
          (`self.ResetCombat`)
          (`KismetSystemLibrary.RetriggerableDelay` 0.7)
          (set `self.isRolling` false)
          (goto _label :!via `Reset`)))
      (elif (!= (`KismetMathLibrary.VSize` (`self.GetVelocity`)) 0.0)
        (`/Engine/EditorBlueprintResources/StandardMacros.DoOnce` false :!label _label_2
          (:`Completed`
            (set `self.isRolling` true)
            (`self.PlayAnimMontage` "/Game/GKnight/Animation/Swordman_Montage/Roll/A_SW_Roll_Forward_Montage.A_SW_Roll_Forward_Montage")
            (`self.ResetCombat`)
            (`KismetSystemLibrary.RetriggerableDelay` 0.7)
            (set `self.isRolling` false)
            (goto _label_2 :!via `Reset`)))))))

(event `InputAction|Block`
  (params (Key :type "Key Structure"))
  ;[1 1 1] Block
  (:`Pressed`
    (if (and (not (`self.isRolling`)) (`self.IsWeaponEquiped`))
      (set `self.isBlocking` true)
      (bind _output_get (set `self.Max Walk Speed` 120.0))
      (`self.ChangePlayerWalkspeed` _output_get)))
  (:`Released`
    (set `self.isBlocking` false)
    (`self.ResetCombat`)
    (bind _output_get_2 (set `self.Max Walk Speed` 300.0))
    (`self.ChangePlayerWalkspeed` _output_get_2)))

(event `InputAction|LightAttack`
  (params (Key :type "Key Structure"))
  ;[1 1 1] LightCombo
  (:`Pressed`
    (if (`self.IsWeaponEquiped`)
      (if (and (not (`self.IsAttacking`)) (not (`self.isRolling`)))
        (set `self.IsAttacking` true)
        (`self.PlayAnimMontage` (`.LightAttack1_2_7FC050B8404F28B54859079894C82680` (break `/Game/Blueprints/Struct/Struct_LighAttacksAnimation` (`self.LighAttacks`))))
        (`/Game/Blueprints/Weapon/BP_Sword.PlayerAttacking` (`self.CastedWeaponObject`)) ; Called this so that damage is only Applied when Player is Attacking
        (else
          (set `self.IsChainAttack` true))))))

(event `ExecuteLightChainAttack`
  ;[1 1 1] LightCombo
  (`/Game/Blueprints/Weapon/BP_Sword.PlayerAttacking` (`self.CastedWeaponObject`)) ; Called this so that damage is only Applied when Player is Attacking
  (`/Engine/EditorBlueprintResources/StandardMacros.IncrementInt` (`self.ComboAttackPointer`)
    (:`  `
      (if (>= (`self.ComboAttackPointer`) 4)
        (set `self.ComboAttackPointer` 0))
      (switch `int` (`self.ComboAttackPointer`)
        (:`0`
          (`self.PlayAnimMontage` (`.LightAttack1_2_7FC050B8404F28B54859079894C82680` (break `/Game/Blueprints/Struct/Struct_LighAttacksAnimation` (`self.LighAttacks`)))))
        (:`1`
          (`self.PlayAnimMontage` (`.LightAttack2_4_A499AFD542A3130BEF095A8C771315E5` (break `/Game/Blueprints/Struct/Struct_LighAttacksAnimation` (`self.LighAttacks`)))))
        (:`2`
          (`self.PlayAnimMontage` (`.LightAttack3_6_614291064167A15CF8C70EB946E53118` (break `/Game/Blueprints/Struct/Struct_LighAttacksAnimation` (`self.LighAttacks`)))))
        (:`3`
          (`self.PlayAnimMontage` (`.LightAttack4_8_49BD640349C4477DCDDAA18D42C9DC5A` (break `/Game/Blueprints/Struct/Struct_LighAttacksAnimation` (`self.LighAttacks`)))))))))

(fn `ChangePlayerWalkspeed`
  (params (WalkSpeed :type "Float (double-precision)"))
  (set `CharacterMovementComponent.MaxWalkSpeed` WalkSpeed (`self.CharacterMovement`))
  (return))

(fn `ChooseRollAnimation`
  (params (Forward :type "Float (double-precision)") (Right :type "Float (double-precision)"))
  (locals (RollLocalForward :type "Float (double-precision)") (RollLocalRight :type "Float (double-precision)"))
  (set `local.RollLocalForward` Forward)
  (set `local.RollLocalRight` Right)
  (if (and (== (`local.RollLocalForward`) 0.0) (== (`local.RollLocalRight`) 0.0))
    (set `self.RollAnimation` "/Game/GKnight/Animation/Swordman_Montage/Avoid/A_SW_Avoid_Backward_Montage.A_SW_Avoid_Backward_Montage")
    (`self.PlayAnimMontage` (`self.RollAnimation`) 1.2 :!label _label)
    (return)
    (elif (and (>= (`local.RollLocalForward`) 0.0) (== (`local.RollLocalRight`) 0.0))
      (set `self.RollAnimation` "/Game/GKnight/Animation/Swordman_Montage/Roll/A_SW_Roll_Forward_Montage.A_SW_Roll_Forward_Montage")
      (goto _label)
      (elif (and (== (`local.RollLocalForward`) 0.0) (>= (`local.RollLocalRight`) 0.0))
        (set `self.RollAnimation` "/Game/GKnight/Animation/Swordman_Montage/Roll/A_SW_Roll_Right_Montage.A_SW_Roll_Right_Montage")
        (goto _label)
        (elif (and (<= (`local.RollLocalForward`) 0.0) (== (`local.RollLocalRight`) 0.0))
          (set `self.RollAnimation` "/Game/GKnight/Animation/Swordman_Montage/Roll/A_SW_Roll_Backward_Montage.A_SW_Roll_Backward_Montage")
          (goto _label)
          (elif (and (== (`local.RollLocalForward`) 0.0) (<= (`local.RollLocalRight`) 0.0))
            (set `self.RollAnimation` "/Game/GKnight/Animation/Swordman_Montage/Roll/A_SW_Roll_Left_Montage.A_SW_Roll_Left_Montage")
            (goto _label)
            (elif (and (>= (`local.RollLocalForward`) 0.0) (>= (`local.RollLocalRight`) 0.0))
              (set `self.RollAnimation` "/Game/GKnight/Animation/Swordman_Montage/Roll/A_SW_Roll_ForwardRight_Montage.A_SW_Roll_ForwardRight_Montage")
              (goto _label)
              (elif (and (<= (`local.RollLocalForward`) 0.0) (>= (`local.RollLocalRight`) 0.0))
                (set `self.RollAnimation` "/Game/GKnight/Animation/Swordman_Montage/Roll/A_SW_Roll_BackwardRight_Montage.A_SW_Roll_BackwardRight_Montage")
                (goto _label)
                (elif (and (<= (`local.RollLocalForward`) 0.0) (<= (`local.RollLocalRight`) 0.0))
                  (set `self.RollAnimation` "/Game/GKnight/Animation/Swordman_Montage/Roll/A_SW_Roll_BackwardLeft_Montage.A_SW_Roll_BackwardLeft_Montage")
                  (goto _label)
                  (elif (and (>= (`local.RollLocalForward`) 0.0) (<= (`local.RollLocalRight`) 0.0))
                    (set `self.RollAnimation` "/Game/GKnight/Animation/Swordman_Montage/Roll/A_SW_Roll_ForwardLeft_Montage.A_SW_Roll_ForwardLeft_Montage")
                    (goto _label)))))))))))

(fn `GetCharacterRef`
  (returns (MyCharacterRef :type "/Game/Blueprints/Character/BP_MyCharacter Object Reference"))
  (return null))

(fn `GetDamageAnimPointer`
  (returns (DamageAnimation :type Integer))
  (return (`self.ComboAttackPointer`)))

(fn `GetDesiredDirectionForRoll`
  (returns (Forward :type "Float (double-precision)") (Right :type "Float (double-precision)"))
  (return (`self.InputAxisForward`) (`self.InputAxisRight`)))

(fn `GetGKnightCharacterRef`
  (returns (GKnightRef :type "/Game/Blueprints/Character/BP_GKnightCharacter Object Reference"))
  (return self))

(fn `GetGknightEnemyRef`
  (returns (EnemyCharacterRef :type "/Game/Blueprints/Emeny/Character/Parent/BP_AI_Enemy_Parent Object Reference"))
  (return null))

(fn `Play Block Animation`
  (if (and (`self.isBlocking`) (not (`self.isRolling`)) (not (`self.IsAttacking`)))
    (bind _output_get (set `self.BlockAnimation` "/Game/GKnight/Animation/Swordman_Montage/Blocking/A_SW_Blocking_Montage.A_SW_Blocking_Montage"))
    (`self.PlayAnimMontage` _output_get 2.0)
    (else
      (`self.StopBlockAnimation`))))

(fn `ResetCombat`
  (set `self.IsAttacking` false)
  (set `self.IsChainAttack` false)
  (set `self.ComboAttackPointer` 0)
  (`/Game/Blueprints/Weapon/BP_Sword.PlayerNotAttackiing` (`self.CastedWeaponObject`))
  (return))

(fn `StopBlockAnimation`
  (`self.StopAnimMontage` (`self.BlockAnimation`)))

(fn `TogglePlayerInput`
  (params (ToggleInput :type Boolean))
  (if ToggleInput
    (`self.EnableInput` self (`GameplayStatics.GetPlayerController` 0))
    (else
      (`self.DisableInput` self (`GameplayStatics.GetPlayerController` 0))))
  (return))

(fn `UserConstructionScript`)