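; Player character Blueprint that handles camera look input and supplies a desired movement direction.
; Turn and look axes drive controller yaw and pitch, with rate-based variants scaled by delta time.
; GetDesiredMovement combines forward and right inputs relative to control yaw into a normalized vector, without applying movement here.
; Tick resets actor rotation to yaw only, working around a root motion capsule rotation bug.
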(event `self.ReceiveTick`
  (params (DeltaSeconds :type "Float (single-precision)"))
  (bind (_returnvalue_roll _returnvalue_pitch _returnvalue_yaw) (`KismetMathLibrary.BreakRotator` (`self.K2_GetActorRotation`)))
  ;[1 1 1] to fix root motion capsule rotation bug
  (`self.K2_SetActorRotation` (`KismetMathLibrary.MakeRotator` 0.0 0.0 _returnvalue_yaw)))

(event `InputAxis|Turn`
  (params (AxisValue :type "Float (single-precision)"))
  (`self.AddControllerYawInput` AxisValue))

(event `InputAxis|LookUp`
  (params (AxisValue :type "Float (single-precision)"))
  (`self.AddControllerPitchInput` AxisValue))

(event `InputAxis|TurnRate`
  (params (AxisValue :type "Float (single-precision)"))
  (`self.AddControllerYawInput` (* AxisValue (`GameplayStatics.GetWorldDeltaSeconds`) (`self.TurnRate`))))

(event `InputAxis|LookUpRate`
  (params (AxisValue :type "Float (single-precision)"))
  (`self.AddControllerPitchInput` (* AxisValue (`GameplayStatics.GetWorldDeltaSeconds`) (`self.LookupRate`))))

(fn `GetCharacterRef`
  (returns (MyCharacterRef :type "/Game/Blueprints/Character/BP_MyCharacter Object Reference"))
  (return self))

(fn `GetDesiredMovement`
  (returns (DesiredVelocity :type "Vector Structure"))
  (bind (_returnvalue_roll _returnvalue_pitch _returnvalue_yaw) (`KismetMathLibrary.BreakRotator` (`self.GetControlRotation`)))
  (return (`KismetMathLibrary.Normal` (+ (* (`KismetMathLibrary.GetForwardVector` (`KismetMathLibrary.MakeRotator` 0.0 0.0 _returnvalue_yaw)) (`self.GetInputAxisValue`)) (* (`KismetMathLibrary.GetRightVector` (`KismetMathLibrary.MakeRotator` 0.0 0.0 _returnvalue_yaw)) (`self.GetInputAxisValue`))))))

(fn `UserConstructionScript`)