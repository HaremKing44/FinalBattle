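; BP_AudioManager is an audio manager Blueprint that plays one of three sound cues: main menu, environment or battle.
; PlaySound spawns the cue chosen by Selector as a 2D sound and stores it in CurrentSound, without stopping any previous one.
; Separate events step Selector up or down within clamped bounds, and stop, pause, unpause or briefly fade CurrentSound.
; Changing Selector takes effect only on the next PlaySound call.
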(event `/Game/Blueprints/Interface/BPI_AudioManager.PlaySound`
  (bind _returnvalue (`GameplayStatics.SpawnSound2D` (select `int` (`self.Selector`) :`0` "/Game/Sound/SoundCue/Music/SC_MainMenu.SC_MainMenu" :`1` "/Game/Sound/SoundCue/SFX/SC_Environment.SC_Environment" :`2` "/Game/Sound/SoundCue/Music/SC_Battle.SC_Battle" :!type "SoundCue Object Reference") 1.0 1.0 0.0 null))
  (set `self.CurrentSound` _returnvalue))

(event `/Game/Blueprints/Interface/BPI_AudioManager.StopSound`
  (`AudioComponent.Stop` (`self.CurrentSound`)))

(event `/Game/Blueprints/Interface/BPI_AudioManager.PauseSound`
  (`AudioComponent.SetPaused` (`self.CurrentSound`) true))

(event `IncreaseSelector`
  (bind _result (`/Engine/EditorBlueprintResources/StandardMacros.IncrementInt` (`self.Selector`))
    (:`  `
      (set `self.Selector` (`KismetMathLibrary.Clamp` _result 0 2)))))

(event `/Game/Blueprints/Interface/BPI_AudioManager.UnpauseSound`
  (`AudioComponent.SetPaused` (`self.CurrentSound`) false))

(event `DecreaseSelector`
  (bind _result (`/Engine/EditorBlueprintResources/StandardMacros.DecrementInt` (`self.Selector`))
    (:`  `
      (set `self.Selector` (`KismetMathLibrary.Clamp` _result 0 2)))))

(event `/Game/Blueprints/Interface/BPI_AudioManager.FadeInSound`
  (`AudioComponent.FadeIn` (`self.CurrentSound`) 0.5 1.0 0.0 "Linear"))

(event `/Game/Blueprints/Interface/BPI_AudioManager.FadeOutSound`
  (`AudioComponent.FadeOut` (`self.CurrentSound`) 0.5 0.0 "Linear"))

(fn `UserConstructionScript`)