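; Parent Blueprint for enemy AI that turns perception updates into Blackboard target and line-of-sight state.
; A successful sense stores the actor as target, flags line of sight and cancels any pending loss timer.
; A failed sense starts a short one-shot timer that clears both, giving a grace period before the target is lost.
; UpdateTargetLocation writes the target's position to the Blackboard but is not called here.
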(event `self.ReceiveBeginPlay`
  (set `self.OurBlackboard` (`AIBlueprintHelperLibrary.GetBlackboard` null)))

(event `self.AIPerception.OnTargetPerceptionUpdated`
  (params (Actor :type "Actor Object Reference") (Stimulus :type "AIStimulus Structure"))
  (set `self.TargetRef` Actor)
  (if (`.bSuccessfullySensed` (break `AIStimulus` Stimulus))
    (`KismetSystemLibrary.K2_ClearAndInvalidateTimerHandle` (`self.UpdateTargetLocationTimer`))
    (`BlackboardComponent.SetValueAsBool` (`self.OurBlackboard`) (`self.BB_HasLineOfSight`) true)
    (`BlackboardComponent.SetValueAsObject` (`self.OurBlackboard`) (`self.BB_Target`) (`self.TargetRef`))
    (else
      (bind _returnvalue (`KismetSystemLibrary.K2_SetTimerDelegate` (delegate `TargetLost`) 5.0))
      (set `self.UpdateTargetLocationTimer` _returnvalue))))

(event `TargetLost`
  (`BlackboardComponent.SetValueAsBool` (`self.OurBlackboard`) (`self.BB_HasLineOfSight`) false)
  (`BlackboardComponent.SetValueAsObject` (`self.OurBlackboard`) (`self.BB_Target`) null))

(fn `UpdateTargetLocation`
  (`BlackboardComponent.SetValueAsVector` (`self.OurBlackboard`) (`self.BB_TargetLocation`) (`self.K2_GetActorLocation` (`self.TargetRef`))))

(fn `UserConstructionScript`)