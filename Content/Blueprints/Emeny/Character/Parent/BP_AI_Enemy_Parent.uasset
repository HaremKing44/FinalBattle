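; Parent character for sword-wielding AI enemies that patrol, fight the player and can drop a key item or relic on death.
; Perception sets blackboard target and engagement keys, with a timer to lose the target, while spline points feed patrol locations.
; It spawns a socketed sword and handles montage combos, blocking, heavy-hit stuns and hit reactions.
; Death ragdolls the body, activates drop FX and enables an overlap pickup prompt that notifies a door opener once collected.
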(event `self.ReceiveBeginPlay`
  ;[1 1 1] Event BeginPlay
  (`SceneComponent.K2_DetachFromComponent` (`self.MyPath`) "KeepWorld" "KeepWorld" "KeepWorld" true)
  (set `self.MaxPathPoint` (`SplineComponent.GetNumberOfSplinePoints` (`self.MyPath`)))
  (set `self.OurBlackboard` (`AIBlueprintHelperLibrary.GetBlackboard` null))
  (bind _returnvalue (`|SpawnActorFromClass` (`self.WeaponClass`) (`SceneComponent.GetSocketTransform` (`self.Mesh`) "SwordHolderSocket" "RTS_World") "Undefined" "OverrideRootScale" null null))
  (bind _output_get (set `self.WeaponObject` _returnvalue))
  (`self.K2_AttachToComponent` _output_get (`self.Mesh`) "SwordHolderSocket" "SnapToTarget" "SnapToTarget" "SnapToTarget" true)
  (bind _asbp_sword (cast `/Game/Blueprints/Weapon/BP_Sword` (`self.WeaponObject`)))
  (bind _output_get_2 (set `self.CastedSowrdObject` _asbp_sword))
  (`/Game/Blueprints/Weapon/BP_Sword.GetSwordParentActor` _output_get_2 self)
  (`BlackboardComponent.SetValueAsBool` (`self.OurBlackboard`) (`self.BB_IsWeaponEquip`) false)
  (`ActorComponent.Deactivate` (`self.AfterDeath_FX`))
  (set `self.TotalHealth` (`self.Health`))
  (if (and (not (`self.CanDropItem`)) (not (`self.CanDropFinalItem`)))
    (`ActorComponent.K2_DestroyComponent` (`self.Box`))))

(event `self.AIPerception.OnTargetPerceptionUpdated`
  (params (Actor :type "Actor Object Reference") (Stimulus :type "AIStimulus Structure"))
  (if (`self.ActorHasTag` Actor "Player")
    (if (`.bSuccessfullySensed` (break `AIStimulus` Stimulus))
      (`KismetSystemLibrary.K2_ClearAndInvalidateTimerHandle` (`self.UpdateTargetLocationTimer`))
      (bind _output_get (set `self.isEngaged` true))
      (`BlackboardComponent.SetValueAsBool` (`self.OurBlackboard`) (`self.BB_HasLineOfSight`) _output_get)
      (bind _gknightref (message `/Game/Blueprints/Interface/BPI_GetGKightCharacterRef.GetGKnightCharacterRef` (`GameplayStatics.GetPlayerCharacter` 0)))
      (`BlackboardComponent.SetValueAsObject` (`self.OurBlackboard`) (`self.BB_Target`) _gknightref)
      (set `CharacterMovementComponent.MaxWalkSpeed` 300.0 (`self.CharacterMovement`))
      (`SceneComponent.SetVisibility` (`self.HealthWidget`) true false)
      (else
        (bind _returnvalue (`KismetSystemLibrary.K2_SetTimerDelegate` (delegate `TargetLost`) 5.0))
        (set `self.UpdateTargetLocationTimer` _returnvalue)))))

(event `TargetLost`
  (bind _output_get (set `self.isEngaged` false))
  (`BlackboardComponent.SetValueAsBool` (`self.OurBlackboard`) (`self.BB_HasLineOfSight`) _output_get)
  (`BlackboardComponent.SetValueAsObject` (`self.OurBlackboard`) (`self.BB_Target`) null)
  (set `CharacterMovementComponent.MaxWalkSpeed` 95.0 (`self.CharacterMovement`))
  (`SceneComponent.SetVisibility` (`self.HealthWidget`) false false))

(event `/Game/Blueprints/Interface/BPI_ApplyDamage.TakeDamage`
  (params (isHeavyAttack :type Boolean))
  ;[1 1 1] Apply Damage to self
  (`/Engine/EditorBlueprintResources/StandardMacros.DoOnce` false :!label _label
    (:`Completed`
      (if (and (`self.isBlocking`) isHeavyAttack)
        (`self.PlayAnimMontage` "/Game/GKnight/Animation/Swordman_Montage/Blocking/A_SW_Blocking_Attack_Montage.A_SW_Blocking_Attack_Montage" 0.5)
        (bind _output_get (set `self.isStun` true))
        (`BlackboardComponent.SetValueAsBool` (`self.OurBlackboard`) (`self.BB_isStun`) _output_get)
        (`|ExecutionSequence`
          (:`then_0`
            (`KismetSystemLibrary.RetriggerableDelay` 3.0)
            (bind _output_get_2 (set `self.isStun` false))
            (`BlackboardComponent.SetValueAsBool` (`self.OurBlackboard`) (`self.BB_isStun`) _output_get_2))
          (:`then_1`
            (`KismetSystemLibrary.RetriggerableDelay` 0.4)
            (goto _label :!via `Reset`)))
        (else
          (if (not (`self.isBlocking`))
            _
            (elif (`self.isAttacking`)
              _
              (else
                (`self.PlayAnimMontage` "/Game/GKnight/Animation/Swordman_Montage/Blocking/A_SW_Blocking_Hit_Montage.A_SW_Blocking_Hit_Montage")
                (goto _label :!via `Reset`))))
          (bind _output_get_3 (set `self.isBeingHit` true))
          (`BlackboardComponent.SetValueAsBool` (`self.OurBlackboard`) (`self.BB_IsBeingHit`) _output_get_3)
          (if (not (`self.isEngaged`))
            (bind _output_get_4 (set `self.isEngaged` true))
            (`BlackboardComponent.SetValueAsBool` (`self.OurBlackboard`) (`self.BB_HasLineOfSight`) _output_get_4)
            (`SceneComponent.SetVisibility` (`self.HealthWidget`) true false))
          (if (> (`self.Health`) 0.0)
            (bind _output_get_5 (set `self.Health` (`KismetMathLibrary.FClamp` (- (`self.Health`) 10.0) 0.0 (`self.TotalHealth`))))
            (`self.UpdateHeathBar` _output_get_5)
            (if (== (`self.Health`) 0.0)
              (`PrimitiveComponent.SetCollisionEnabled` (`/Game/Blueprints/Weapon/BP_Sword.SwordBoxCollison` (`self.CastedSowrdObject`)) "NoCollision")
              (`CharacterMovementComponent.DisableMovement` (`self.CharacterMovement`))
              (`Controller.UnPossess` (`self.GetController`))
              (`PrimitiveComponent.SetSimulatePhysics` (`self.Mesh`) true)
              (`ActorComponent.K2_DestroyComponent` (`self.CapsuleComponent`))
              (`SceneComponent.SetVisibility` (`self.HealthWidget`) false false)
              (`self.DropKey`)
              (`self.DropFinalItem`)
              (else
                (`self.PlayAnimMontage` "/Game/GKnight/Animation/Swordman_Montage/Damage/A_SW_Damage_Fast_Montage.A_SW_Damage_Fast_Montage")
                (`self.ResetCombat`)
                (`KismetSystemLibrary.RetriggerableDelay` 0.4)
                (bind _output_get_6 (set `self.isBeingHit` false))
                (`BlackboardComponent.SetValueAsBool` (`self.OurBlackboard`) (`self.BB_IsBeingHit`) _output_get_6)
                (goto _label :!via `Reset`)))))))))

(event `Patrol`
  ;[1 1 1] Patroling System
  (bind _iswalkback (`self.GetIsWalkBack`))
  (bind _pathpointlocation (`self.GetPathPointLocation` _iswalkback))
  (`BlackboardComponent.SetValueAsVector` (`self.OurBlackboard`) (`self.BB_PathPointLocation`) _pathpointlocation))

(event `DropFinalItem`
  (if (`self.CanDropFinalItem`)
    (`ActorComponent.Activate` (`self.AfterDeath_FX`) false)))

(event `DropKey`
  (if (`self.CanDropItem`)
    (`ActorComponent.Activate` (`self.AfterDeath_FX`) false)))

(event `ToggleWeaponEquip`
  ;[1 1 1] Toggle Equip Weapon
  (if (not (`self.isWeaponEquip`))
    (set `self.isWeaponEquip` true)
    (`BlackboardComponent.SetValueAsBool` (`self.OurBlackboard`) (`self.BB_IsWeaponEquip`) (`self.isWeaponEquip`))
    (`self.PlayAnimMontage` "/Game/GKnight/Animation/Swordman_Montage/Equip/A_SW_Equip_Montage.A_SW_Equip_Montage" 1.4)
    (bind _gknightref (message `/Game/Blueprints/Interface/BPI_GetGKightCharacterRef.GetGKnightCharacterRef` (`GameplayStatics.GetPlayerCharacter` 0)))
    (`AIController.K2_SetFocus` (`AIBlueprintHelperLibrary.GetAIController` self) _gknightref)
    (else
      (set `self.isWeaponEquip` false)
      (`BlackboardComponent.SetValueAsBool` (`self.OurBlackboard`) (`self.BB_IsWeaponEquip`) (`self.isWeaponEquip`))
      (`self.PlayAnimMontage` "/Game/GKnight/Animation/Swordman_Montage/Equip/A_SW_Unequip_Trim_Montage.A_SW_Unequip_Trim_Montage" 1.4)
      (`AIController.K2_ClearFocus` (`AIBlueprintHelperLibrary.GetAIController` self)))))

(event `PerformAttack`
  ;[1 1 1] Attack Logic
  (if (not (`self.isAttacking`))
    (set `self.isAttacking` true)
    (`self.PlayAnimMontage` "/Game/GKnight/Animation/Swordman_Montage/Attack/A_SW_Attack_01_Montage.A_SW_Attack_01_Montage")
    (`/Game/Blueprints/Weapon/BP_Sword.AIAttacking` (`self.CastedSowrdObject`))
    (`self.CheckTargetCanBlock`)
    (else
      (set `self.isChainAttack` true))))

(event `ExecuteLightChainAttack`
  ;[1 1 1] Attack Logic
  (`/Game/Blueprints/Weapon/BP_Sword.AIAttacking` (`self.CastedSowrdObject`))
  (`self.CheckTargetCanBlock`)
  (`/Engine/EditorBlueprintResources/StandardMacros.IncrementInt` (`self.ComboAttackPointer`)
    (:`  `
      (if (>= (`self.ComboAttackPointer`) 4)
        (set `self.ComboAttackPointer` 0))
      (switch `int` (`self.ComboAttackPointer`)
        (:`0`
          (`self.PlayAnimMontage` (`.LightAttack1_2_7FC050B8404F28B54859079894C82680` (break `/Game/Blueprints/Struct/Struct_LighAttacksAnimation` (`self.AttackAnim`)))))
        (:`1`
          (`self.PlayAnimMontage` (`.LightAttack2_4_A499AFD542A3130BEF095A8C771315E5` (break `/Game/Blueprints/Struct/Struct_LighAttacksAnimation` (`self.AttackAnim`)))))
        (:`2`
          (`self.PlayAnimMontage` (`.LightAttack3_6_614291064167A15CF8C70EB946E53118` (break `/Game/Blueprints/Struct/Struct_LighAttacksAnimation` (`self.AttackAnim`)))))
        (:`3`
          (`self.PlayAnimMontage` (`.LightAttack4_8_49BD640349C4477DCDDAA18D42C9DC5A` (break `/Game/Blueprints/Struct/Struct_LighAttacksAnimation` (`self.AttackAnim`)))))))))

(event `Block`
  ;[1 1 1] Block
  (set `self.isBlocking` true))

(event `Unblock`
  ;[1 1 1] Block
  (set `self.isBlocking` false))

(event `self.Box.OnComponentBeginOverlap`
  (params (OverlappedComponent :type "PrimitiveComponent Object Reference") (OtherActor :type "Actor Object Reference") (OtherComp :type "PrimitiveComponent Object Reference") (OtherBodyIndex :type Integer) (bFromSweep :type Boolean) (SweepResult :type "HitResult Structure (by ref)"))
  (if (== (`self.Health`) 0.0)
    (if (`self.ActorHasTag` OtherActor "Player")
      (if (`self.CanDropFinalItem`)
        (bind _gknightref (message `/Game/Blueprints/Interface/BPI_GetGKightCharacterRef.GetGKnightCharacterRef` OtherActor))
        (set `/Game/Blueprints/Character/BP_GKnightCharacter.canPickFinalItem` true _gknightref)
        (else
          (bind _gknightref_2 (message `/Game/Blueprints/Interface/BPI_GetGKightCharacterRef.GetGKnightCharacterRef` OtherActor))
          (set `/Game/Blueprints/Character/BP_GKnightCharacter.canPickItem` true _gknightref_2)))
      (`self.UpdateMessageUI`)
      (`SceneComponent.SetVisibility` (`self.MessageWidget`) true false)
      (bind _returnvalue (`KismetSystemLibrary.K2_SetTimer` null "DeleteDropItem" 0.2 true))
      (set `self.DeleteDropItemTimer` _returnvalue))))

(event `self.Box.OnComponentEndOverlap`
  (params (OverlappedComponent :type "PrimitiveComponent Object Reference") (OtherActor :type "Actor Object Reference") (OtherComp :type "PrimitiveComponent Object Reference") (OtherBodyIndex :type Integer))
  (if (`self.ActorHasTag` OtherActor "Player")
    (if (`self.CanDropFinalItem`)
      (bind _gknightref (message `/Game/Blueprints/Interface/BPI_GetGKightCharacterRef.GetGKnightCharacterRef` OtherActor))
      (set `/Game/Blueprints/Character/BP_GKnightCharacter.canPickFinalItem` false _gknightref)
      (else
        (bind _gknightref_2 (message `/Game/Blueprints/Interface/BPI_GetGKightCharacterRef.GetGKnightCharacterRef` OtherActor))
        (set `/Game/Blueprints/Character/BP_GKnightCharacter.canPickItem` false _gknightref_2)))
    (`SceneComponent.SetVisibility` (`self.MessageWidget`) false false)
    (if (`KismetSystemLibrary.K2_IsValidTimerHandle` (`self.DeleteDropItemTimer`))
      (`KismetSystemLibrary.K2_ClearAndInvalidateTimerHandle` (`self.DeleteDropItemTimer`)))))

(fn `CheckTargetCanBlock`
  (bind _returnvalue (`GameplayStatics.GetPlayerCharacter` 0))
  (if (`KismetMathLibrary.InRange_FloatFloat` (`KismetMathLibrary.Dot_VectorVector` (`self.GetActorForwardVector`) (`self.GetActorForwardVector` (`GameplayStatics.GetPlayerCharacter` 0))) -1.0 -0.7)
    (message `/Game/Blueprints/Interface/BPI_SetCanBlock.SetCanBlock` _returnvalue true)
    (return)
    (else
      (message `/Game/Blueprints/Interface/BPI_SetCanBlock.SetCanBlock` _returnvalue false)
      (return))))

(fn `DeleteDropItem`
  (bind _gknightref (message `/Game/Blueprints/Interface/BPI_GetGKightCharacterRef.GetGKnightCharacterRef` (`GameplayStatics.GetPlayerCharacter` 0)))
  (if (or (`/Game/Blueprints/Character/BP_GKnightCharacter.HaveKey` _gknightref) (`/Game/Blueprints/Character/BP_GKnightCharacter.haveFinalItem` _gknightref))
    (`/Game/Blueprints/Environment/Unlock/Parent/BP_Unlock_Parent.CheckKeyStatus` (`self.DoorOpener`))
    (`ActorComponent.K2_DestroyComponent` (`self.Box`))
    (`ActorComponent.Deactivate` (`self.AfterDeath_FX`))
    (`SceneComponent.SetVisibility` (`self.MessageWidget`) false false)
    (if (`KismetSystemLibrary.K2_IsValidTimerHandle` (`self.DeleteDropItemTimer`))
      (`KismetSystemLibrary.K2_ClearAndInvalidateTimerHandle` (`self.DeleteDropItemTimer`))
      (return))))

(fn `GetGKnightCharacterRef`
  (returns (GKnightRef :type "/Game/Blueprints/Character/BP_GKnightCharacter Object Reference"))
  (return null))

(fn `GetGknightEnemyRef`
  (returns (EnemyCharacterRef :type "/Game/Blueprints/Emeny/Character/Parent/BP_AI_Enemy_Parent Object Reference"))
  (return self))

(fn `GetIsWalkBack`
  (returns (isWalkBack :type Boolean))
  (if (== (`self.PathIndex`) (- (`self.MaxPathPoint`) 1))
    (bind _output_get (set `self.isWalkingBack` true))
    (return _output_get)
    (elif (== (`self.PathIndex`) 0)
      (bind _output_get_2 (set `self.isWalkingBack` false))
      (return _output_get_2))))

(fn `GetPathPointLocation`
  (params (isWalkingBack :type Boolean))
  (returns (PathPointLocation :type "Vector Structure"))
  (bind _pathindex (`self.PathIndex`))
  (if isWalkingBack
    (`/Engine/EditorBlueprintResources/StandardMacros.DecrementInt` _pathindex
      (:`  `
        _))
    (else
      (`/Engine/EditorBlueprintResources/StandardMacros.IncrementInt` _pathindex
        (:`  `
          _))))
  (return (`SplineComponent.GetLocationAtSplinePoint` (`self.MyPath`) (`self.PathIndex`) "World")))

(fn `GetStrafLocation`
  (returns (NewStrafLoction :type "Vector Structure"))
  (bind _mesh (`self.Mesh`))
  (bind _mesh_2 (`self.Mesh`))
  (if (== (`KismetMathLibrary.RandomIntegerInRange` 0 1) 0)
    (return (+ (`SceneComponent.K2_GetComponentLocation` _mesh_2) (* (`SceneComponent.GetForwardVector` _mesh_2) 50.0) (* (`SceneComponent.GetRightVector` _mesh_2) 150.0)))
    (else
      (return (+ (`SceneComponent.K2_GetComponentLocation` _mesh) (* (`SceneComponent.GetForwardVector` _mesh) 50.0) (* (`SceneComponent.GetRightVector` _mesh) -150.0))))))

(fn `ResetCombat`
  (set `self.IsAttacking` false)
  (set `self.IsChainAttack` false)
  (set `self.ComboAttackPointer` 0)
  (`/Game/Blueprints/Weapon/BP_Sword.AINotAttacking` (`self.CastedSowrdObject`))
  (return))

(fn `UpdateHeathBar`
  (params (Health :type "Float (double-precision)"))
  (message `/Game/Blueprints/Interface/BPI_UIUpdate.UpdateHealthBar` (`WidgetComponent.GetUserWidgetObject` (`self.HealthWidget`)) (/ Health (`self.TotalHealth`)))
  (return))

(fn `UpdateMessageUI`
  (if (`self.CanDropFinalItem`)
    (set `self.UI_MessageText` "Press [E] to pick Relic")
    (else
      (bind _output_get (set `self.UI_MessageText` "Press [E] to pick Item"))))
  (message `/Game/Blueprints/Interface/BPI_UIUpdate.UpdateMessageText` (`WidgetComponent.GetUserWidgetObject` (`self.MessageWidget`)) _output_get))

(fn `UserConstructionScript`)