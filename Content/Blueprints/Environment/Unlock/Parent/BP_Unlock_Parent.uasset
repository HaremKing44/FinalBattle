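; Parent Blueprint for unlock points where a player carrying a key or final item can activate the object.
; Box overlap enables key use, shows a prompt and starts a looping timer that polls for key use.
; On use, it plays item FX, removes the trigger and opens the linked door, except for the final item.
; CheckKeyStatus briefly blends the camera to this actor while freezing player movement.
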(event `self.ReceiveBeginPlay`
  (`ActorComponent.Deactivate` (`self.ItemPut_FX`)))

(event `CheckKeyStatus`
  (bind _returnvalue (`GameplayStatics.GetPlayerController` 0))
  (bind _gknightref (message `/Game/Blueprints/Interface/BPI_GetGKightCharacterRef.GetGKnightCharacterRef` (`GameplayStatics.GetPlayerCharacter` 0)))
  (if (or (`/Game/Blueprints/Character/BP_GKnightCharacter.HaveKey` _gknightref) (`/Game/Blueprints/Character/BP_GKnightCharacter.haveFinalItem` _gknightref))
    (`PlayerController.SetViewTargetWithBlend` _returnvalue self 1.0 "VTBlend_Linear" 0.0 false)
    (bind _charactermovement (`Character.CharacterMovement` _gknightref))
    (`CharacterMovementComponent.DisableMovement` _charactermovement)
    (`KismetSystemLibrary.Delay` 2.0)
    (`PlayerController.SetViewTargetWithBlend` _returnvalue _gknightref 1.0 "VTBlend_Linear" 0.0 false)
    (`KismetSystemLibrary.Delay` 1.0)
    (`CharacterMovementComponent.SetMovementMode` _charactermovement "MOVE_Walking" 0)))

(event `self.BoxCollision.OnComponentBeginOverlap`
  (params (OverlappedComponent :type "PrimitiveComponent Object Reference") (OtherActor :type "Actor Object Reference") (OtherComp :type "PrimitiveComponent Object Reference") (OtherBodyIndex :type Integer) (bFromSweep :type Boolean) (SweepResult :type "HitResult Structure (by ref)"))
  (if (`self.ActorHasTag` OtherActor "Player")
    (bind _gknightref (message `/Game/Blueprints/Interface/BPI_GetGKightCharacterRef.GetGKnightCharacterRef` OtherActor))
    (if (or (`/Game/Blueprints/Character/BP_GKnightCharacter.HaveKey` _gknightref) (`/Game/Blueprints/Character/BP_GKnightCharacter.haveFinalItem` _gknightref))
      (set `/Game/Blueprints/Character/BP_GKnightCharacter.canUseKey` true _gknightref)
      (`SceneComponent.SetVisibility` (`self.MessageWidget`) true false)
      (`self.UpdateMessageUI`)
      (bind _returnvalue (`KismetSystemLibrary.K2_SetTimer` null "OpenGate" 0.2 true))
      (set `self.OpenGateTimer` _returnvalue))))

(event `self.BoxCollision.OnComponentEndOverlap`
  (params (OverlappedComponent :type "PrimitiveComponent Object Reference") (OtherActor :type "Actor Object Reference") (OtherComp :type "PrimitiveComponent Object Reference") (OtherBodyIndex :type Integer))
  (if (`self.ActorHasTag` OtherActor "Player")
    (bind _gknightref (message `/Game/Blueprints/Interface/BPI_GetGKightCharacterRef.GetGKnightCharacterRef` OtherActor))
    (set `/Game/Blueprints/Character/BP_GKnightCharacter.canUseKey` false _gknightref)
    (`SceneComponent.SetVisibility` (`self.MessageWidget`) false false)))

(fn `OpenGate`
  (bind _gknightref (message `/Game/Blueprints/Interface/BPI_GetGKightCharacterRef.GetGKnightCharacterRef` (`GameplayStatics.GetPlayerCharacter` 0)))
  (if (`/Game/Blueprints/Character/BP_GKnightCharacter.isKeyUsed` _gknightref)
    (if (not (`/Game/Blueprints/Character/BP_GKnightCharacter.haveFinalItem` _gknightref))
      (`/Game/Blueprints/Environment/Doors/BP_OpenableDoor.OpenDoor` (`self.OpenableDoor`)))
    (`ActorComponent.Activate` (`self.ItemPut_FX`) false)
    (if (`KismetSystemLibrary.K2_IsValidTimerHandle` (`self.OpenGateTimer`))
      (`KismetSystemLibrary.K2_ClearAndInvalidateTimerHandle` (`self.OpenGateTimer`))
      (`ActorComponent.K2_DestroyComponent` (`self.BoxCollision`))
      (else
        (return)))
    (else
      (return))))

(fn `UpdateMessageUI`
  (bind _output_get (set `self.UI_MessageText` "Press [E] to Activate"))
  (message `/Game/Blueprints/Interface/BPI_UIUpdate.UpdateMessageText` (`WidgetComponent.GetUserWidgetObject` (`self.MessageWidget`)) _output_get))

(fn `UserConstructionScript`)