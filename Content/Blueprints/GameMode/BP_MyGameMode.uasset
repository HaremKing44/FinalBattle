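; Game mode that tracks whether a level is running and opens the pause menu.
; A setter event and a getter function expose the running flag, which gates the Pause input action.
; Pressing Pause creates a new main menu widget, switches it to a fixed page and plays its pause fade-in.
; It then gives the UI input focus, shows the cursor and pauses the game.
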(event `self.ReceiveBeginPlay`)

(event `/Game/Blueprints/Interface/BPI_GameMode.SetLevelRunning`
  (params (isLevelRunning :type Boolean))
  (set `self.isLevelRunning` isLevelRunning))

(event `InputAction|Pause`
  (params (Key :type "Key Structure"))
  (bind _returnvalue (`GameplayStatics.GetPlayerController` 0))
  (:`Pressed`
    (if (`self.isLevelRunning`)
      (bind _returnvalue_2 (`|CreateWidget` "/Game/UI/MainMenu/UI_MainMenu.UI_MainMenu_C" (`GameplayStatics.GetPlayerController` 0)))
      (`UserWidget.AddToViewport` _returnvalue_2 0)
      (`WidgetSwitcher.SetActiveWidgetIndex` (`/Game/UI/MainMenu/UI_MainMenu.WidgetSwitcher_88` _returnvalue_2) 4)
      (`UserWidget.PlayAnimation` _returnvalue_2 (`/Game/UI/MainMenu/UI_MainMenu.PauseMenuFadeIn` _returnvalue_2) 0.0 1 "Forward" 2.0 false)
      (`WidgetBlueprintLibrary.SetInputMode_UIOnlyEx` _returnvalue _returnvalue_2)
      (set `PlayerController.bShowMouseCursor` true _returnvalue)
      (`GameplayStatics.SetGamePaused` true))))

(fn `GetLevelRunning`
  (returns (isLevelRunning :type Boolean))
  (return (`self.isLevelRunning`)))

(fn `UserConstructionScript`)